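; ConjurableShield_BP is a shield actor for the ability weapons that shows a visual impact reaction when an AbilityProjectile hits its mesh.
; On hit, it writes the hit location into the shield material and spawns an electric hit particle oriented by the impact normal.
; Four timelines then restart together, animating two pairs of radius and WDM scale material parameters to ripple the surface from that point.
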(event `self.ShieldMesh.OnComponentHit`
  (params (HitComponent :type "PrimitiveComponent Object Reference") (OtherActor :type "Actor Object Reference") (OtherComp :type "PrimitiveComponent Object Reference") (NormalImpulse :type "Vector Structure") (Hit :type "HitResult Structure (by ref)"))
  (bind _shieldmaterial (`self.ShieldMaterial`))
  (cast `AbilityProjectile` OtherActor)
  (`MaterialInstanceDynamic.SetVectorParameterValue` (`self.ShieldMaterial`) "Location" (`KismetMathLibrary.Conv_VectorToLinearColor` Hit_Location))
  ;[1 1 1] Hit Particle
  (`GameplayStatics.SpawnEmitterAtLocation` "/Game/Assets/VisualFX/MageShield/P_ElectricShieldHit.P_ElectricShieldHit" Hit_ImpactPoint (`KismetMathLibrary.MakeRotFromZ` (* Hit_ImpactNormal -1.0)) (0.5 0.5 0.5))
  ;[1 1 1] Hit Animation
  (`|ExecutionSequence`
    (:`then_0`
      (bind (_direction _radius) (`Timeline|Timeline` :!via `PlayFromStart`)
        (:`Update`
          (`MaterialInstanceDynamic.SetScalarParameterValue` _shieldmaterial "Radius" (* _radius 100.0)))))
    (:`then_1`
      (bind (_direction_2 _wdm) (`Timeline|Timeline_0` :!via `PlayFromStart`)
        (:`Update`
          (`MaterialInstanceDynamic.SetScalarParameterValue` _shieldmaterial "WDM Scale" (* _wdm 20.0)))))
    (:`then_2`
      (bind (_direction_3 _radius_2) (`Timeline|Timeline_1` :!via `PlayFromStart`)
        (:`Update`
          (`MaterialInstanceDynamic.SetScalarParameterValue` _shieldmaterial "Radius 2" (* _radius_2 130.0)))))
    (:`then_3`
      (bind (_direction_4 _wdm_2) (`Timeline|Timeline_2` :!via `PlayFromStart`)
        (:`Update`
          (`MaterialInstanceDynamic.SetScalarParameterValue` _shieldmaterial "WDM Scale 2" (* _wdm_2 15.0)))))))

(fn `UserConstructionScript`)
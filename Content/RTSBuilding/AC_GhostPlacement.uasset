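; Actor component for RTS building that is meant to make a ghost structure follow the mouse cursor during placement.
; Each tick it sets the owner's location from PlayerControllerMouseToWorldLocation, whose cursor trace with 100-unit X/Y grid snapping and fixed height appears unconnected to any output.
; CheckIsPlacing reads the owning A_GhostStructure's PlacingGhost flag, but its result does not gate the move.
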(event `self.ReceiveTick`
  (params (DeltaSeconds :type "Float (single-precision)"))
  (bind _asa_ghost_structure (cast `/Game/RTSBuilding/A_GhostStructure` (`self.GetOwner`)))
  (if (`/Game/RTSBuilding/A_GhostStructure.PlacingGhost` _asa_ghost_structure)
    (`Actor.K2_SetActorLocation` (`self.GetOwner` self) (`self.PlayerControllerMouseToWorldLocation`) false false)))